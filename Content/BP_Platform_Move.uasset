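; Moving platform that shuttles back and forth between two points at constant speed.
; BeginPlay turns the P1 and P2 offsets into world targets relative to the starting location and heads for P2 first.
; Tick moves the actor with VInterpToConstant without sweeping, then uses distance tolerances to flip the target.
; The tolerances differ, so it turns back slightly short of P2 but travels closer to P1.
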(event EventTick
  (params (DeltaSeconds :type Float%20%28single-precision%29))
  (Transformation|SetActorLocation (Math|Interpolation|VInterptoConstant (Transformation|GetActorLocation) (Variables|Default|GetObjectiveLocal) DeltaSeconds (Variables|Default|GetSpeed)) false false)
  (if (Utilities|Operators|EqualEqual (Transformation|GetActorLocation) (Variables|Default|GetObjectiveLocal) 5.0)
    (if (Utilities|Operators|EqualEqual (Variables|Default|GetObjective1) (Transformation|GetActorLocation) 1.0)
      (Variables|Default|SetObjectiveLocal (Variables|Default|GetObjective2))
      (else
        (Variables|Default|SetObjectiveLocal (Variables|Default|GetObjective1))))))

(event EventBeginPlay
  (bind _output_get (Variables|Default|SetObjective2 (+ (Variables|Default|GetP2) (Transformation|GetActorLocation))))
  (Variables|Default|SetObjectiveLocal _output_get)
  (Variables|Default|SetObjective1 (+ (Variables|Default|GetP1) (Transformation|GetActorLocation))))

(fn ConstructionScript)